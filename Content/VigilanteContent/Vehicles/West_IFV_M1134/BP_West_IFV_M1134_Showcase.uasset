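; Showcase Blueprint for the West IFV M1134 vehicle, exposing its appearance and moving parts to generic button, checkbox and slider controls.
; Each indexed control event forwards its value to a named setter for skin, damaged model, wheels, turret, launcher, hatches, lights or mirrors.
; The setters are not defined here, the construction script only calls its parent, and Tick is unused.
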(event `/Game/VigilanteContent/Shared/Blueprints/Showcase/Interfaces/BP_ShowcaseControlsInterface.SetButtonsVariable0`
  (params (NewIndex :type Integer))
  ;[1 1 1] Skin variant
  (`self.SetSkinType` (`KismetMathLibrary.Conv_IntToDouble` NewIndex)))

(event `/Game/VigilanteContent/Shared/Blueprints/Showcase/Interfaces/BP_ShowcaseControlsInterface.SetCheckboxVariable0`
  (params (NewState :type Boolean))
  ;[1 1 1] Damaged model visibility
  (`self.SetShowDamaged` NewState))

(event `/Game/VigilanteContent/Shared/Blueprints/Showcase/Interfaces/BP_ShowcaseControlsInterface.SetSliderVariable0`
  (params (NewValue :type "Float (single-precision)"))
  ;[1 1 1] Speed
  (`self.SetWheelSpeed` NewValue))

(event `/Game/VigilanteContent/Shared/Blueprints/Showcase/Interfaces/BP_ShowcaseControlsInterface.SetSliderVariable1`
  (params (NewValue :type "Float (single-precision)"))
  ;[1 1 1] Wheel Angle
  (`self.SetWheelAngle` NewValue))

(event `/Game/VigilanteContent/Shared/Blueprints/Showcase/Interfaces/BP_ShowcaseControlsInterface.SetSliderVariable2`
  (params (NewValue :type "Float (single-precision)"))
  ;[1 1 1] Turret rotation
  (`self.Set Turrent Rotation` NewValue))

(event `/Game/VigilanteContent/Shared/Blueprints/Showcase/Interfaces/BP_ShowcaseControlsInterface.SetSliderVariable3`
  (params (NewValue :type "Float (single-precision)"))
  ;[1 1 1] Luncher Rotation
  (`self.Set Launcher Rotation` NewValue))

(event `/Game/VigilanteContent/Shared/Blueprints/Showcase/Interfaces/BP_ShowcaseControlsInterface.SetSliderVariable4`
  (params (NewValue :type "Float (single-precision)"))
  ;[1 1 1] Hatches
  (`self.SetTopHatchesRotation` NewValue))

(event `/Game/VigilanteContent/Shared/Blueprints/Showcase/Interfaces/BP_ShowcaseControlsInterface.SetSliderVariable5`
  (params (NewValue :type "Float (single-precision)"))
  ;[1 1 1] Lights
  (`self.SetLightsEmissivity` NewValue))

(event `/Game/VigilanteContent/Shared/Blueprints/Showcase/Interfaces/BP_ShowcaseControlsInterface.SetSliderVariable6`
  (params (NewValue :type "Float (single-precision)"))
  ;[1 1 1] Mirrors base rotation
  (`self.SetMirrorsBaseRotation` NewValue))

(event `/Game/VigilanteContent/Shared/Blueprints/Showcase/Interfaces/BP_ShowcaseControlsInterface.SetSliderVariable7`
  (params (NewValue :type "Float (single-precision)"))
  ;[1 1 1] Mirrors rotation
  (`self.SetMirrorsRotation` NewValue))

(fn `UserConstructionScript`
  (`parent.UserConstructionScript`))